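; Base HUD Blueprint that puts the interact and main HUD widgets on screen at BeginPlay and opens the equipment, bag and loot box windows.
; Each open event acts only for a valid local controller, lazily creating its widget on a fixed Z-order layer or re-showing the cached one.
; It then initializes the window with the controller, plus the loot box where relevant, shows the cursor and switches to focused UI-only input.
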(event `self.ReceiveBeginPlay`
  (bind _returnvalue (`|CreateWidget` "/Game/UI/HUD/WB_Interact_Window.WB_Interact_Window_C"))
  (`UserWidget.AddToViewport` _returnvalue 0)
  (bind _returnvalue_2 (`|CreateWidget` "/Game/UI/HUD/WB_HUD_Window.WB_HUD_Window_C"))
  (`UserWidget.AddToViewport` _returnvalue_2 1))

(event `OpenInventory`
  (params (PlayerController :type "PlayerController Object Reference"))
  (bind _player_controller (`self.Player Controller`))
  (bind _output_get (set `self.Player Controller` PlayerController))
  (`/Engine/EditorBlueprintResources/StandardMacros.IsValid` _output_get
    (:`Is Valid`
      (if (`Controller.IsLocalController` _output_get)
        (`self.InventoryWidget`
          (:`then`
            (`Widget.SetVisibility` (`self.InventoryWidget`) "SelfHitTestInvisible"))
          (:`else`
            (bind _returnvalue (`|CreateWidget` "/Game/UI/Inventoty/WB_EquipmentWindow.WB_EquipmentWindow_C" (`self.Player Controller`)))
            (bind _output_get_2 (set `self.InventoryWidget` _returnvalue))
            (`UserWidget.AddToViewport` _output_get_2 2)))
        (`/Game/UI/Inventoty/WB_EquipmentWindow.InitParams` _output_get_2 _player_controller)
        (set `PlayerController.bShowMouseCursor` true _player_controller)
        (set `UserWidget.bIsFocusable` true _output_get_2)
        (`WidgetBlueprintLibrary.SetInputMode_UIOnlyEx` _player_controller _output_get_2)))))

(event `OpenBag`
  (params (`Player Controller` :type "PlayerController Object Reference"))
  (bind _player_controller (`self.Player Controller`))
  (bind _output_get (set `self.Player Controller` `Player Controller`))
  (`/Engine/EditorBlueprintResources/StandardMacros.IsValid` _output_get
    (:`Is Valid`
      (if (`Controller.IsLocalController` _output_get)
        (`self.BagWidget`
          (:`then`
            (`Widget.SetVisibility` (`self.BagWidget`) "SelfHitTestInvisible"))
          (:`else`
            (bind _returnvalue (`|CreateWidget` "/Game/UI/Inventoty/WB_Bag_Window.WB_Bag_Window_C" (`self.Player Controller`)))
            (bind _output_get_2 (set `self.BagWidget` _returnvalue))
            (`UserWidget.AddToViewport` _output_get_2 3)))
        (`/Game/UI/Inventoty/WB_Bag_Window.InitParams` _output_get_2 _player_controller)
        (set `PlayerController.bShowMouseCursor` true _player_controller)
        (set `UserWidget.bIsFocusable` true _output_get_2)
        (`WidgetBlueprintLibrary.SetInputMode_UIOnlyEx` _player_controller _output_get_2)))))

(event `OpenLootBox`
  (params (`Player Controller` :type "PlayerController Object Reference") (Self_0 :type "/Game/BluePrints/Inventory/PickUps/BP_Chest Object Reference"))
  (bind _lootboxwidget (`self.LootBoxWidget`))
  (bind _player_controller (`self.Player Controller`))
  (`/Engine/EditorBlueprintResources/StandardMacros.IsValid` Self_0
    (:`Is Valid`
      (bind _output_get (set `self.Player Controller` `Player Controller`))
      (`/Engine/EditorBlueprintResources/StandardMacros.IsValid` _output_get
        (:`Is Valid`
          (if (`Controller.IsLocalController` _output_get)
            (`self.LootBoxWidget`
              (:`then`
                (`Widget.SetVisibility` (`self.LootBoxWidget`) "SelfHitTestInvisible"))
              (:`else`
                (bind _returnvalue (`|CreateWidget` "/Game/UI/Inventoty/WB_LootBox_Window.WB_LootBox_Window_C" (`self.Player Controller`)))
                (set `self.LootBoxWidget` _returnvalue)
                (`UserWidget.AddToViewport` _returnvalue 5)))
            (`/Game/UI/Inventoty/WB_LootBox_Window.Init` _lootboxwidget _player_controller Self_0)
            (set `PlayerController.bShowMouseCursor` true _player_controller)
            (set `UserWidget.bIsFocusable` true _lootboxwidget)
            (`WidgetBlueprintLibrary.SetInputMode_UIOnlyEx` _player_controller _lootboxwidget)))))))

(fn `UserConstructionScript`)