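; Base player controller that bridges inventory, bag and loot box interactions to the HUD and loot boxes.
; Enhanced Input actions open inventory or bag, and loot box opening runs on the local controller only, all through a lazily cached BP_BaseHUD reference.
; Taking items and closing boxes forward to the loot box's server-named functions.
; WaitForInventoryReadiness polls each tick until the item manager and quick bar are valid.
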(event `EnhancedInput|/Game/BluePrints/Input/Actions/AI_Open_Inventory`
  (params (ActionValue :type Boolean) (ElapsedSeconds :type "Float (double-precision)") (TriggeredSeconds :type "Float (double-precision)") (InputAction :type "InputAction Object Reference" :default "/Game/BluePrints/Input/Actions/AI_Open_Inventory.AI_Open_Inventory"))
  (:`Started`
    (`self.As BP Base HUD`
      (:`then`
        _)
      (:`else`
        (bind _asbp_base_hud (cast `/Game/BluePrints/BP_BaseHUD` (`self.GetHUD`)))
        (bind _output_get (set `self.As BP Base HUD` _asbp_base_hud))))
    (`/Game/BluePrints/BP_BaseHUD.OpenInventory` _output_get self)))

(event `OpenLootBox`
  (params (LootBox :type "/Game/BluePrints/Inventory/PickUps/BP_Chest Object Reference"))
  (`/Engine/EditorBlueprintResources/StandardMacros.IsValid` LootBox
    (:`Is Valid`
      (if (`self.IsLocalController`)
        (`self.As BP Base HUD`
          (:`then`
            _)
          (:`else`
            (bind _asbp_base_hud (cast `/Game/BluePrints/BP_BaseHUD` (`self.GetHUD`)))
            (bind _output_get (set `self.As BP Base HUD` _asbp_base_hud))))
        (`/Game/BluePrints/BP_BaseHUD.OpenLootBox` _output_get self LootBox)))))

(event `LootBoxTakeItem`
  (params (LootBox :type "/Game/BluePrints/Inventory/PickUps/BP_Chest Object Reference") (Index :type Integer))
  (`/Engine/EditorBlueprintResources/StandardMacros.IsValid` LootBox
    (:`Is Valid`
      (`/Game/BluePrints/Inventory/PickUps/BP_Chest.TakeItem_Serv` LootBox Index))))

(event `CloseLootBox`
  (params (LootBox :type "/Game/BluePrints/Inventory/PickUps/BP_Chest Object Reference"))
  (`/Engine/EditorBlueprintResources/StandardMacros.IsValid` LootBox
    (:`Is Valid`
      (`/Game/BluePrints/Inventory/PickUps/BP_Chest.CloseLootBox_Ser` LootBox))))

(event `EnhancedInput|/Game/BluePrints/Input/Actions/AI_Open_Bag`
  (params (ActionValue :type Boolean) (ElapsedSeconds :type "Float (double-precision)") (TriggeredSeconds :type "Float (double-precision)") (InputAction :type "InputAction Object Reference" :default "/Game/BluePrints/Input/Actions/AI_Open_Bag.AI_Open_Bag"))
  (:`Started`
    (`self.As BP Base HUD`
      (:`then`
        _)
      (:`else`
        (bind _asbp_base_hud (cast `/Game/BluePrints/BP_BaseHUD` (`self.GetHUD`)))
        (bind _output_get (set `self.As BP Base HUD` _asbp_base_hud))))
    (`/Game/BluePrints/BP_BaseHUD.OpenBag` _output_get self)))

(fn `UserConstructionScript`)