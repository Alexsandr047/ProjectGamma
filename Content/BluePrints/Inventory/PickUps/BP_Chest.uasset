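; BP_Chest is an interactable loot chest that opens a loot box through the interacting player's controller.
; InitLoot rolls its items on the server from a PGItemsSubsystem loot list.
; TakeItem removes an entry, notifies listeners and, on authority, passes it to the player's quick bar component, while OnRep keeps clients updated.
; Closing toggles a replicated flag whose OnRep destroys an empty chest or removes open/interact gameplay effects on authority.
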(event `self.ReceiveBeginPlay`
  (`parent.ReceiveBeginPlay`))

(event `self.ReceiveTick`
  (params (DeltaSeconds :type "Float (single-precision)"))
  (`parent.ReceiveTick` DeltaSeconds))

(event `TakeItem_Serv`
  (params (Index :type Integer))
  (`self.Take Item` Index))

(event `CloseLootBox_Ser`
  (set `self.bClose` (not (`self.bClose`))))

(fn `Close`
  (if (> (`KismetArrayLibrary.Array_Length` (`self.Items`)) 0)
    (`/Engine/EditorBlueprintResources/ActorMacros.Switch Has Authority`
      (:`Authority`
        (`AbilitySystemComponent.RemoveActiveGameplayEffect` (`AbilitySystemBlueprintLibrary.GetAbilitySystemComponent` self) (`self.GE_OpenObject`) -1)
        (`AbilitySystemComponent.RemoveActiveGameplayEffect` (`AbilitySystemBlueprintLibrary.GetAbilitySystemComponent` self) (`self.GE_InteractingHandle`) -1)))
    (else
      (`self.K2_DestroyActor`))))

(fn `GetItems`
  (returns (Items :type "Array of ModifiableItemBase Structure"))
  (return (`self.Items`)))

(fn `InitLoot`
  (`/Engine/EditorBlueprintResources/ActorMacros.Switch Has Authority`
    (:`Authority`
      (bind (_items _returnvalue) (`PG_ItemsSubsystem.MakeLootDropList` (subsystem `PG_ItemsSubsystem`) "LootDrop_01"))
      (if _returnvalue
        (set `self.Items` _items)))))

(fn `InteractLogic`
  (params (`Interacting Actor` :type "Actor Object Reference"))
  (`/Engine/EditorBlueprintResources/StandardMacros.IsValid` `Interacting Actor`
    (:`Is Valid`
      (bind _asbp_base_player_controller (cast `/Game/BluePrints/BP_BasePlayerController` (`self.GetInstigatorController` `Interacting Actor`)))
      (bind _output_get (set `self.Player Controller` _asbp_base_player_controller))
      (`/Game/BluePrints/BP_BasePlayerController.OpenLootBox` _output_get self))))

(fn `OnRep_bClose`
  (`self.Close`))

(fn `OnRep_Items`
  (`self.UpdateItems`))

(fn `Take Item`
  (params (Index :type Integer))
  (locals (Item :type "ModifiableItemBase Structure"))
  (bind _player_controller (`self.Player Controller`))
  (bind _returnvalue (`KismetArrayLibrary.Array_Length` (`self.Items`)))
  (bind _returnvalue_2 (`self.GetComponentByClass` _player_controller "/Script/ProjectGamma.PG_QuickBarComponent"))
  (if (and (not (>= (`local.Index`) _returnvalue)) (> _returnvalue (`local.Index`)))
    (set `local.Item` (`|GetArrayItem` (`self.Items`) (`local.Index`)))
    (`KismetArrayLibrary.Array_Remove` (`self.Items`) (`local.Index`))
    (`self.UpdateItems`)
    (`/Engine/EditorBlueprintResources/ActorMacros.Switch Has Authority`
      (:`Authority`
        (`/Engine/EditorBlueprintResources/StandardMacros.IsValid` _returnvalue_2
          (:`Is Valid`
            (`/Engine/EditorBlueprintResources/StandardMacros.IsValid` (`self.GetComponentByClass` _player_controller "/Script/CharacterInitializationSystem.CIS_ItemManagerComponent")
              (:`Is Valid`
                (`PG_QuickBarComponent.InitItemsToInventory` _returnvalue_2 (`|MakeArray` (`local.Item`)))))))))))

(fn `UserConstructionScript`
  (`parent.UserConstructionScript`))