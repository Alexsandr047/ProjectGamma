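; Base interactable pickup actor that uses GAS to track its interaction state, with InitLoot and InteractLogic as override hooks.
; The server applies GE_Interacting on pre-interact, removes it on cancel or completion, then applies GE_ObjectOpen from the interactor and runs InteractLogic, which destroys the actor by default.
; Availability is blocked by matching gameplay tags, and pre-interact syncs as OnlyClientWait.
; An async tag listener starts on BeginPlay, but its handlers are empty.
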(event `self.ReceiveBeginPlay`
  (set `self.Interaction Component` (`self.StaticMesh`))
  (`self.InitLoot`)
  (bind (_asynctaskproxy _tag) (`AsyncTaskGameplayTagAddedRemoved.ListenForGameplayTagAddedOrRemoved` null (`self.ListenTags`))
    (:`then`
      (set `self.ListenForTagAddRemovedTask` _asynctaskproxy))
    (:`OnTagAdded`
      (bind _returnvalue (== _tag (`self.OpenTag`)))
      (if _returnvalue
        _))
    (:`OnTagRemoved`
      (if _returnvalue
        _))))

(event `self.PreInteract`
  (params (InteractingActor :type "Actor Object Reference") (InteractionComponent :type "PrimitiveComponent Object Reference"))
  (bind _returnvalue (`AbilitySystemBlueprintLibrary.GetAbilitySystemComponent` self))
  ;[1 1 1] PreInteract
  (if (== InteractionComponent (`self.Interaction Component`))
    (`/Engine/EditorBlueprintResources/ActorMacros.Switch Has Authority`
      (:`Authority`
        (bind _returnvalue_2 (`AbilitySystemComponent.BP_ApplyGameplayEffectToSelf` _returnvalue "/Game/BluePrints/Ability/GE_Interacting.GE_Interacting_C" 0.0 (`AbilitySystemComponent.MakeEffectContext` _returnvalue)))
        (set `self.GE_InteractingHandle` _returnvalue_2)))))

(event `self.PostInteract`
  (params (InteractingActor :type "Actor Object Reference") (InteractionComponent :type "PrimitiveComponent Object Reference"))
  (bind _returnvalue (`AbilitySystemBlueprintLibrary.GetAbilitySystemComponent` InteractingActor))
  ;[1 1 1] PostInteract
  (if (== InteractionComponent (`self.Interaction Component`))
    (`/Engine/EditorBlueprintResources/ActorMacros.Switch Has Authority`
      (:`Authority`
        (bind _returnvalue_2 (`AbilitySystemComponent.BP_ApplyGameplayEffectToTarget` _returnvalue "/Game/BluePrints/Inventory/PickUps/GE_ObjectOpen.GE_ObjectOpen_C" (`AbilitySystemBlueprintLibrary.GetAbilitySystemComponent` self) 0.0 (`AbilitySystemComponent.MakeEffectContext` _returnvalue)))
        (set `self.GE_OpenObject` _returnvalue_2)
        (`AbilitySystemComponent.RemoveActiveGameplayEffect` (`AbilitySystemBlueprintLibrary.GetAbilitySystemComponent` self) (`self.GE_InteractingHandle`) -1)
        (`self.InteractLogic` InteractingActor)))))

(event `CancelInteraction_1`
  (params (InteractionComponent :type "PrimitiveComponent Object Reference"))
  ;[1 1 1] CancelInteraction - Player stops interacting (releases input early, stunned, etc).
  (if (== InteractionComponent (`self.Interaction Component`))
    (`/Engine/EditorBlueprintResources/ActorMacros.Switch Has Authority`
      (:`Authority`
        (`AbilitySystemComponent.RemoveActiveGameplayEffect` (`AbilitySystemBlueprintLibrary.GetAbilitySystemComponent` self) (`self.GE_InteractingHandle`) -1)))))

(event `self.ReceiveEndPlay`
  (params (EndPlayReason :type "EEndPlayReason Enum" :default "Destroyed"))
  (bind _listenfortagaddremovedtask (`self.ListenForTagAddRemovedTask`)
    (:`then`
      (`AsyncTaskGameplayTagAddedRemoved.EndTask` _listenfortagaddremovedtask))
    (:`else`)))

(event `self.ReceiveTick`
  (params (DeltaSeconds :type "Float (single-precision)")))

(fn `GetInteractionDuration`
  (params (InteractionComponent :type "PrimitiveComponent Object Reference"))
  (returns (ReturnValue :type "Float (single-precision)"))
  (if (== InteractionComponent (`self.Interaction Component`))
    (return (`self.OpenInteractionDuration`))
    (else
      (return 0.0))))

(fn `GetPostInteractSyncType`
  (params (InteractionComponent :type "PrimitiveComponent Object Reference"))
  (returns (bShouldSync :type Boolean) (Type :type "EAbilityTaskNetSyncType Enum"))
  (if (== InteractionComponent (`self.Interaction Component`))
    (return false "OnlyServerWait")
    (else
      (return false "OnlyServerWait"))))

(fn `GetPreInteractSyncType`
  (params (InteractionComponent :type "PrimitiveComponent Object Reference"))
  (returns (bShouldSync :type Boolean) (Type :type "EAbilityTaskNetSyncType Enum"))
  (if (== InteractionComponent (`self.Interaction Component`))
    (return true "OnlyClientWait")
    (else
      (return false "OnlyServerWait"))))

(fn `InitLoot`)

(fn `InteractLogic`
  (params (`Interacting Actor` :type "Actor Object Reference"))
  ;[1 1 1] BaseLogicForOverride
  (`self.K2_DestroyActor`))

(fn `IsAvailableForInteraction`
  (params (InteractionComponent :type "PrimitiveComponent Object Reference"))
  (returns (ReturnValue :type Boolean))
  (return (and (== InteractionComponent (`self.Interaction Component`)) (not (`GameplayTagAssetInterface.HasAnyMatchingGameplayTags` (`AbilitySystemBlueprintLibrary.GetAbilitySystemComponent` self) (`self.AvailabilityTags`))))))

(fn `UserConstructionScript`)