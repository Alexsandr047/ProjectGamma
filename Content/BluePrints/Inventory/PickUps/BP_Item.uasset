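; BP_Item is an inventory pickup actor whose interaction and loot logic is mostly stubbed out.
; InteractLogic checks the interacting actor for quick bar and item manager components but does nothing with them, then destroys the pickup regardless.
; InitLoot contains only an authority switch with no following logic, and unused items subsystem getters remain in the graphs.
; The default event nodes are disabled, and the construction script only calls its parent.
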(fn `InitLoot`
  (`/Engine/EditorBlueprintResources/ActorMacros.Switch Has Authority`))

(fn `InteractLogic`
  (params (`Interacting Actor` :type "Actor Object Reference"))
  (bind _interacting_actor (`local.Interacting Actor`))
  (`|ExecutionSequence`
    (:`then_0`
      (`/Engine/EditorBlueprintResources/StandardMacros.IsValid` (`self.GetComponentByClass` _interacting_actor "/Script/ProjectGamma.PG_QuickBarComponent")
        (:`Is Valid`
          (`/Engine/EditorBlueprintResources/StandardMacros.IsValid` (`self.GetComponentByClass` _interacting_actor "/Script/CharacterInitializationSystem.CIS_ItemManagerComponent")))))
    (:`then_1`
      (`self.K2_DestroyActor`))))

(fn `UserConstructionScript`
  (`parent.UserConstructionScript`))