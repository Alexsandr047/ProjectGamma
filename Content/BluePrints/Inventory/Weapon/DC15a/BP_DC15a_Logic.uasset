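; DC-15A weapon logic that decides whether an attachment can be used with the current attachment set.
; GetAttachmentSlots offers Scope, Barrel, Picatiny and Frame slots, adding Laser only when a Picatiny-tagged attachment is present.
; CheckForUseOfAttachment accepts a candidate whose gameplay tags match an available slot hierarchically, unless an existing attachment has identical item tags.
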(fn `CheckForUseOfAttachment`
  (params (AttachmentDefinition :type "Array of CIS_ItemDefinition Object Reference (by ref)") (CheckedAttachmentDefinition :type "CIS_ItemDefinition Object Reference"))
  (returns (ReturnValue :type Boolean))
  (locals (bCanUse :type Boolean))
  (bind _returnvalue (`self.GetAttachmentSlots` AttachmentDefinition))
  (for _array_element _returnvalue
    (if (`BlueprintGameplayTagLibrary.HasTag` (`CIS_ItemDefinition.GetItemTags` (`local.CheckedAttachmentDefinition`)) _array_element)
      (for _array_element_2 (`local.AttachmentDefinition`)
        (if (== (`CIS_ItemDefinition.GetItemTags` _array_element_2) (`CIS_ItemDefinition.GetItemTags` (`local.CheckedAttachmentDefinition`)))
          (return false)))
      (return true)))
  (return false))

(fn `GetAttachmentSlots`
  (params (AttachmentDefinition :type "Array of CIS_ItemDefinition Object Reference (by ref)"))
  (returns (ReturnValue :type "Array of GameplayTag Structure"))
  (locals (SlotsCanUsed :type "Array of GameplayTag Structure"))
  (set `local.SlotsCanUsed` (`|MakeArray` (`self.Scope`) (`self.Barrel`) (`self.Picatiny`) (`self.Frame`)))
  (for _array_element (`local.AttachmentDefinition`)
    (if (`BlueprintGameplayTagLibrary.HasTag` (`CIS_ItemDefinition.GetItemTags` _array_element) (`self.Picatiny`))
      (`KismetArrayLibrary.Array_Add` (`local.SlotsCanUsed`) (`self.Laser`))
      (break)))
  (return (`local.SlotsCanUsed`)))