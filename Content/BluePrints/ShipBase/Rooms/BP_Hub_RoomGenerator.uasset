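; BP_Hub_RoomGenerator is a ship room hub that presents a clickable room panel and serves as a camera view target for clearing or building that room.
; It initializes its WB_RoomPanel widget with room data, retrying on a short delay until the cast succeeds.
; SetViewPanelCamera blends the view to itself, locks its panel, hides the other hubs' panels, and opens clearing or building options in BuildRoomWB by room condition.
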(event `self.ReceiveBeginPlay`)

(event `self.SetRoomData`
  (params (RoomGenerator :type "PG_Hub_RoomGenerator Object Reference"))
  (bind _aswb_room_panel (cast `/Game/UI/ShipBase/WB_RoomPanel` (`WidgetComponent.GetWidget` (`self.Widget`)) :!label _label)
    (:`then`
      (set `self.As WB Room Panel` _aswb_room_panel)
      (`/Game/UI/ShipBase/WB_RoomPanel.InitTypeRoom` (`self.As WB Room Panel`) RoomGenerator))
    (:`CastFailed`
      (`KismetSystemLibrary.Delay` 0.1)
      (goto _label))))

(fn `Hidden Panel`
  (bind _as_wb_room_panel (`self.As WB Room Panel`)
    (:`then`
      (`/Game/UI/ShipBase/WB_RoomPanel.HiddenPanel` _as_wb_room_panel))
    (:`else`)))

(fn `Init`
  (params (`Player Controller` :type "PlayerController Object Reference") (RoomGenerators :type "Array of /Game/BluePrints/ShipBase/Rooms/BP_Hub_RoomGenerator Object Reference"))
  (set `self.Player Controller` `Player Controller`)
  (set `self.RoomGenerators` RoomGenerators))

(fn `SetViewPanelCamera`
  (`|ExecutionSequence`
    (:`then_0`
      (`PlayerController.SetViewTargetWithBlend` (`self.Player Controller`) self 1.0 "VTBlend_Linear" 0.0 false)
      (for _array_element (`self.RoomGenerators`)
        (if (!= _array_element self)
          (`self.Hidden Panel` _array_element)
          (else
            (`/Game/UI/ShipBase/WB_RoomPanel.LockPanel` (`self.As WB Room Panel`))))))
    (:`then_1`
      (`self.GetRoomCondition`
        (:`Debris`
          (`/Game/UI/ShipBase/WB_RoomBuilding_Window.ShowClearingParm` (`self.Build Room WB`) self))
        (:`Empty`
          (`/Game/UI/ShipBase/WB_RoomBuilding_Window.ShowBuildingParam` (`self.Build Room WB`) self))))))

(fn `ShowWidget`
  (params (`Build Room WB` :type "/Game/UI/ShipBase/WB_RoomBuilding_Window Object Reference"))
  (bind _as_wb_room_panel (`self.As WB Room Panel`))
  (`|ExecutionSequence`
    (:`then_0`
      (`self.As WB Room Panel`
        (:`then`
          _)
        (:`else`
          (bind _aswb_room_panel (cast `/Game/UI/ShipBase/WB_RoomPanel` (`WidgetComponent.GetWidget` (`self.Widget`))))
          (set `self.As WB Room Panel` _aswb_room_panel)))
      (`/Game/UI/ShipBase/WB_RoomPanel.ShowPanel` _as_wb_room_panel)
      (add `/Game/UI/ShipBase/WB_RoomPanel.ClickRoomPanel` _as_wb_room_panel (`|CreateDelegate` :!event `SetViewPanelCamera`)))
    (:`then_1`
      (`self.Build Room WB`
        (:`then`)
        (:`else`
          (set `self.Build Room WB` `Build Room WB`))))))

(fn `UserConstructionScript`)