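; Main menu player controller that shows the intro logo and authorization window, then reveals the preview character.
; It possesses the preview character, starts client data initialization through the game mode and initializes the quick bar on possession.
; A three-flag gate waits for logo finish, item loading and a short delay before switching the view and removing the logo.
; Entered credentials go to the GameInstance, whose completion callback opens the ship base map unless the tutorial should start.
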(event `self.ReceiveBeginPlay`
  (`|ExecutionSequence`
    (:`then_0`
      (bind _returnvalue (`|CreateWidget` "/Game/UI/MainMenu/WB_MainMenu_Logo.WB_MainMenu_Logo_C"))
      (set `self.Logo` _returnvalue)
      (`UserWidget.AddToViewport` _returnvalue 1)
      (bind _returnvalue_2 (`|CreateWidget` "/Game/UI/MainMenu/WB_AuthorizationMenu_Window.WB_AuthorizationMenu_Window_C"))
      (set `self.Authorization_Menu` _returnvalue_2)
      (`UserWidget.AddToViewport` _returnvalue_2 0)
      (add `/Game/UI/MainMenu/WB_MainMenu_Logo.FinishPlayLogo` _returnvalue (delegate `LogoFinishPlay`))
      (add `/Game/UI/MainMenu/WB_AuthorizationMenu.SetAuthorization` (`/Game/UI/MainMenu/WB_AuthorizationMenu_Window.WB_AuthorizationMenu` (`self.Authorization_Menu`)) (delegate `Autorization`))
      (bind _aspg_game_instance (cast `PG_GameInstance` (`GameplayStatics.GetGameInstance`)))
      (set `self.Game_Instance` _aspg_game_instance)
      (add `PG_GameInstance.AuthorizationComplete` _aspg_game_instance (delegate `CustomEvent`)))
    (:`then_1`
      (bind _returnvalue_3 (`GameplayStatics.GetActorOfClass` "/Game/BluePrints/MainMenu/BP_PreviewCharacter.BP_PreviewCharacter_C"))
      (bind _output_get (set `self.PreviewCharacter` _returnvalue_3))
      (add `/Game/BluePrints/MainMenu/BP_PreviewCharacter.ItemLoaded` _output_get (delegate `ItemLoaded`))
      (`/Engine/EditorBlueprintResources/StandardMacros.IsValid` _output_get
        (:`Is Valid`
          (bind _aspg_main_menu_game_mode (cast `PG_MainMenu_GameMode` (`GameplayStatics.GetGameMode`)))
          (`PG_GameMode.StartPlayerInitializedClientData` _aspg_main_menu_game_mode self)
          (`self.Possess` (`self.PreviewCharacter`))
          (`KismetSystemLibrary.Delay` 2.0)
          (set `self.DefaultTimer` true)
          (`self.Check Character`))))))

(event `CustomEvent`
  (params (bStartTutorial :type Boolean))
  (if (not bStartTutorial)
    (`GameplayStatics.OpenLevel` "/Game/Maps/ShipBase/W_ShipBaseMap")))

(event `LogoFinishPlay`
  (set `self.LogoFinish` true)
  (`self.Check Character`))

(event `Autorization`
  (params (Login :type String) (Password :type String))
  (bind _game_instance (`self.Game_Instance`)
    (:`then`
      (`PG_GameInstance.AuthorizePlayer` _game_instance Login Password))
    (:`else`)))

(event `ItemLoaded`
  (set `self.bItemLoaded` true)
  (`self.Check Character`))

(event `Check Character`
  (if (and (`self.LogoFinish`) (`self.bItemLoaded`) (`self.DefaultTimer`))
    (`self.SetViewTargetWithBlend` (`self.PreviewCharacter`))
    (`Widget.RemoveFromParent` (`self.Logo`))))

(event `self.ReceivePossess`
  (params (PossessedPawn :type "Pawn Object Reference"))
  (bind _pg_quickbar (`self.PG_QuickBar`)
    (:`then`
      (`PG_QuickBarComponent.InitializeClientData` _pg_quickbar))
    (:`else`)))

(fn `UserConstructionScript`)