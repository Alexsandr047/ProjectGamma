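; Main menu preview character that sets up its character preset and starting equipment.
; InitCharacterData runs on authority only, initializing CharacterPresets, then waiting for the controller's item manager and quick bar components.
; The WaitForInventoryReadiness macro retries each tick until all exist.
; AddInitialInventory then binds to the quick bar's item-loaded event and calls InitEquip with the item manager.
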(event `self.InitCharacterData`
  (`/Engine/EditorBlueprintResources/ActorMacros.Switch Has Authority`
    (:`Authority`
      (`PG_CharacterPresets_Component.InitCharacterPreset` (`self.CharacterPresets`))
      (`self.WaitForInventoryReadiness`
        (:`ExecOut`
          (`self.Add Initial Inventory`))))))

(fn `Add Initial Inventory`
  (locals (InventoryManager :type "CIS_ItemManagerComponent Object Reference") (QuickBar :type "PG_QuickBarComponent Object Reference"))
  (bind _returnvalue (`self.GetController`))
  (bind _returnvalue_2 (`self.GetComponentByClass` _returnvalue "/Script/ProjectGamma.PG_QuickBarComponent"))
  (bind _returnvalue_3 (`self.GetComponentByClass` _returnvalue "/Script/CharacterInitializationSystem.CIS_ItemManagerComponent"))
  (`/Engine/EditorBlueprintResources/StandardMacros.IsValid` _returnvalue
    (:`Is Valid`
      (`/Engine/EditorBlueprintResources/StandardMacros.IsValid` _returnvalue_3
        (:`Is Valid`
          (set `local.InventoryManager` _returnvalue_3)
          (`/Engine/EditorBlueprintResources/StandardMacros.IsValid` _returnvalue_2
            (:`Is Valid`
              (bind _output_get (set `local.QuickBar` _returnvalue_2))
              (add `PG_QuickBarComponent.ItemLoaded` _returnvalue_2 (`|CreateDelegate` :!event `Call Item Loaded`))
              (`PG_QuickBarComponent.InitEquip` _output_get (`local.InventoryManager`)))))))))

(fn `Call Item Loaded`
  (`self.ItemLoaded`))

(fn `UserConstructionScript`)