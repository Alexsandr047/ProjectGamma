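; Gameplay ability that equips the weapon in the primary quick bar slot.
; On activation it gets the PG_QuickBarComponent from the controller, fetches the primary slot item and casts it to BP_WeaponInstance.
; It starts that weapon's equip montage, calls OnEquipped immediately rather than on completion, and ends when the montage completes, is interrupted or is cancelled.
; A failed cast stops the graph without ending the ability.
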(event `self.K2_ActivateAbility`
  (set `self.QuickBarComponent` (`Actor.GetComponentByClass` (`self.GetControllerFromActorInfo`) "/Script/ProjectGamma.PG_QuickBarComponent"))
  (bind _weapon (`PG_QuickBarComponent.GetWeaponItem` (`self.QuickBarComponent`) "PrimaryWeaponSlot"))
  (bind _asbp_weapon_instance (cast `/Game/BluePrints/Inventory/Weapon/BP_WeaponInstance` _weapon))
  (set `self.As BP Weapon Instance` _asbp_weapon_instance)
  (`AbilityTask_PlayMontageAndWait.CreatePlayMontageAndWaitProxy` "None" (`/Game/BluePrints/Inventory/Weapon/BP_WeaponInstance.WeaponEquipMontage` (`self.As BP Weapon Instance`))
    (:`then`
      (`PG_WeaponInstance.OnEquipped` (`self.As BP Weapon Instance`)))
    (:`OnCompleted`
      (`self.K2_EndAbility`))
    (:`OnInterrupted`
      (`self.K2_EndAbility` :!label _label))
    (:`OnCancelled`
      (goto _label))))