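; BP_BaseCharacter is a base character Blueprint handling server-authoritative character setup, equipment item use and death cleanup.
; InitCharacterData applies presets, polls each tick until controller, item manager and quick bar exist, then calls AddInitialInventory, whose equip and load nodes are disconnected.
; Item use forwards to the controller's quick bar.
; Death clears quick bar and inventory, then notifies PG_GameMode after a short delay.
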(event `Server_UseItemOnEquipmentSlot`
  (params (EquipSlot :type "EPG_EWeaponSlots Enum" :default "Default") (InventorySlot :type Integer))
  (`self.UseItemOnEquipmentSlot` EquipSlot InventorySlot))

(event `self.ReceivePossessed`
  (params (NewController :type "Controller Object Reference")))

(event `self.InitCharacterData`
  (`/Engine/EditorBlueprintResources/ActorMacros.Switch Has Authority`
    (:`Authority`
      (`PG_CharacterPresets_Component.InitCharacterPreset` (`self.CharacterPresets`))
      (`self.WaitForInventoryReadiness`
        (:`ExecOut`
          (`self.Add Initial Inventory`))))))

(event `self.ReceiveBeginPlay`)

(event `self.K2_OnDeathFinished`)

(event `self.K2_OnReset`)

(event `self.HealthComponent.OnDeathStarted`
  (params (OwningActor :type "Actor Object Reference"))
  (`self.Clear Inventory`)
  (`/Engine/EditorBlueprintResources/ActorMacros.Switch Has Authority`
    (:`Authority`
      (`KismetSystemLibrary.Delay` 0.1)
      (bind _aspg_game_mode (cast `PG_GameMode` (`GameplayStatics.GetGameMode`)))
      (`PG_GameMode.CharacterDied` _aspg_game_mode (`self.GetInstigatorController` OwningActor)))))

(event `self.ReceiveTick`
  (params (DeltaSeconds :type "Float (single-precision)")))

(fn `Add Initial Inventory`
  (locals (InventoryManager :type "CIS_ItemManagerComponent Object Reference") (QuickBar :type "PG_QuickBarComponent Object Reference") (NewLocalVar :type "CIS_ItemDefinition Class Reference" :default "/Script/Engine.BlueprintGeneratedClass'/Game/BluePrints/Inventory/Weapon/DC15a/BP_DC15a.BP_DC15a_C'"))
  (bind _returnvalue (`self.GetController`))
  (bind _returnvalue_2 (`self.GetComponentByClass` _returnvalue "/Script/ProjectGamma.PG_QuickBarComponent"))
  (bind _returnvalue_3 (`self.GetComponentByClass` _returnvalue "/Script/CharacterInitializationSystem.CIS_ItemManagerComponent"))
  (`/Engine/EditorBlueprintResources/ActorMacros.Switch Has Authority`
    (:`Authority`
      (`/Engine/EditorBlueprintResources/StandardMacros.IsValid` _returnvalue
        (:`Is Valid`
          (`/Engine/EditorBlueprintResources/StandardMacros.IsValid` _returnvalue_3
            (:`Is Valid`
              (set `local.InventoryManager` _returnvalue_3)
              (`/Engine/EditorBlueprintResources/StandardMacros.IsValid` _returnvalue_2
                (:`Is Valid`
                  (bind _output_get (set `local.QuickBar` _returnvalue_2)))))))))))

(fn `Clear Inventory`
  (locals (QuickBar :type "PG_QuickBarComponent Object Reference") (InventoryManager :type "CIS_ItemManagerComponent Object Reference"))
  (bind _returnvalue (`self.GetController`))
  (bind _returnvalue_2 (`self.GetComponentByClass` _returnvalue "/Script/ProjectGamma.PG_QuickBarComponent"))
  (bind _returnvalue_3 (`self.GetComponentByClass` _returnvalue "/Script/CharacterInitializationSystem.CIS_ItemManagerComponent"))
  (`/Engine/EditorBlueprintResources/ActorMacros.Switch Has Authority`
    (:`Authority`
      (`/Engine/EditorBlueprintResources/StandardMacros.IsValid` _returnvalue_2
        (:`Is Valid`
          (set `local.QuickBar` _returnvalue_2)
          (`/Engine/EditorBlueprintResources/StandardMacros.IsValid` _returnvalue_3
            (:`Is Valid`
              (set `local.InventoryManager` _returnvalue_3)
              (`|ExecutionSequence`
                (:`then_0`
                  (`PG_QuickBarComponent.RemoveAllItemsFromSlots` (`local.QuickBar`)))
                (:`then_1`
                  (`CIS_ItemManagerComponent.RemoveAllItemFromInventory` (`local.InventoryManager`)))))))))))

(fn `UseItemOnEquipmentSlot`
  (params (EquipSlot :type "EPG_EWeaponSlots Enum" :default "Default") (InventorySlot :type Integer))
  (`/Engine/EditorBlueprintResources/ActorMacros.Switch Has Authority`
    (:`Authority`
      (`PG_QuickBarComponent.UseItemOnEquipmentSlot` (`self.GetComponentByClass` (`self.GetController`) "/Script/ProjectGamma.PG_QuickBarComponent") EquipSlot InventorySlot))))

(fn `UserConstructionScript`)